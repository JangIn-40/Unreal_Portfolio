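; Shared base projectile Blueprint that handles the visual and audio effects of projectile flight and impacts.
; On BeginPlay it attaches the optional flight emitter to the collision box and the fly sound to the root.
; Separate character-hit and world-hit events spawn their own impact emitters and share one impact sound, attached to the projectile at half volume for world hits.
; Hit detection and movement are not scripted in these graphs.
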(event EventBeginPlay
  (Utilities|FlowControl|Sequence
    (:then_0
      (bind _projectilefx (Variables|Default|GetProjectileFX)
        (:then
          (Effects|SpawnEmitterAttached _projectilefx (Variables|Default|GetProjectileCollisionBox) "None" (+ (Transformation|GetActorLocation) (Variables|Default|GetSpawnFXLocationOffset)) (Math|Conversions|RotationFromXVector (Transformation|GetActorForwardVector)) "1.000000,1.000000,1.000000" "KeepWorldPosition"))
        (:else)))
    (:then_1
      (bind _projectileflysound (Variables|Default|GetProjectileFlySound)
        (:then
          (Audio|SpawnSoundAttached _projectileflysound (Variables|Transformation|GetRootComponent) "None" "0, 0, 0" "0, 0, 0" "KeepRelativeOffset" true 0.4 1.0 0.0 0 0))
        (:else)))))

(event Collision|EventActorBeginOverlap
  (params (OtherActor :type Actor%20Object%20Reference)))

(event EventTick
  (params (DeltaSeconds :type Float%20%28single-precision%29)))

(event EventOnSpawnProjectileHitCharacterFX
  (params (HitLocation :type Vector%20%28by%20ref%29 :default "0, 0, 0"))
  (Utilities|FlowControl|Sequence
    (:then_0
      (bind _projectileimpactcharacterfx (Variables|Default|GetProjectileImpactCharacterFX)
        (:then
          (Effects|SpawnEmitteratLocation _projectileimpactcharacterfx HitLocation))
        (:else)))
    (:then_1
      (bind _projectileimpactsound (Variables|Default|GetProjectileImpactSound)
        (:then
          (Audio|PlaySoundatLocation _projectileimpactsound HitLocation "0, 0, 0" 0.5 1.0 0.0 0 0 0 0))
        (:else)))))

(event EventOnSpawnProjectileHitWolrdFX
  (params (HitLocation :type Vector%20%28by%20ref%29 :default "0, 0, 0"))
  (Utilities|FlowControl|Sequence
    (:then_0
      (bind _projectileimpactworldfx (Variables|Default|GetProjectileImpactWorldFX)
        (:then
          (Effects|SpawnEmitteratLocation _projectileimpactworldfx HitLocation))
        (:else)))
    (:then_1
      (bind _projectileimpactsound (Variables|Default|GetProjectileImpactSound)
        (:then
          (Audio|SpawnSoundAttached _projectileimpactsound (Variables|Transformation|GetRootComponent) "None" "0, 0, 0" "0, 0, 0" "KeepRelativeOffset" false 0.5 1.0 0.0 0 0))
        (:else)))))

(fn ConstructionScript)