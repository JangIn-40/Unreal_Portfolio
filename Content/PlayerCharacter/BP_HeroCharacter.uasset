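; Player hero character Blueprint that keeps special ability UI in sync with player state and opens the pause screen.
; BeginPlay sets up async gameplay tag listeners: grounded disables Slam, falling enables it, and low mana disables Slam, ForcePush and Ult.
; Removing low mana sends all three back as activatable with their cooldown tags.
; The pause input async-loads the pause widget class, then adds it to the viewport.
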(event Input|EnhancedActionEvents|EnhancedInputActionIA_PauseMenu
  (params (ActionValue :type Boolean) (ElapsedSeconds :type Float%20%28double-precision%29) (TriggeredSeconds :type Float%20%28double-precision%29) (InputAction :type Input%20Action%20Object%20Reference :default "/Game/PlayerCharacter/Input/Actions/IA_PauseMenu.IA_PauseMenu"))
  (:Started
    (bind _class (Utilities|AsyncLoadClassAsset "/Game/Widget/GameModeWidgets/WBP_PauseScreen.WBP_PauseScreen_C")
      (:Completed
        (bind _asuser_widget (Utilities|Casting|CastToUserWidgetClass _class))
        (bind _returnvalue (UserInterface|CreateWidget _asuser_widget))
        (UserInterface|Viewport|AddtoViewport _returnvalue 0)))))

(event EventBeginPlay
  (Ability|Tasks|WaitGameplayTagAddToActor 0 "(TagName=\"Player.Status.IsGrounded\")"
    (:then
      (Ability|Tasks|WaitGameplayTagAddToActor 0 "(TagName=\"Player.Status.IsFalling\")"
        (:then
          (Ability|Tasks|WaitGameplayTagAddToActor 0 "(TagName=\"Player.Status.LowMana\")"
            (:then
              (Ability|Tasks|WaitGameplayTagRemoveFromActor 0 "(TagName=\"Player.Status.LowMana\")"
                (:Removed
                  (Class|MWBlueprintFunctionLibrary|SendAbilityActivateabletoUI self "(TagName=\"InputTag.SpecialAbility.Slam\")" "(TagName=\"Player.Cooldown.SpecialAbility.Slam\")")
                  (Class|MWBlueprintFunctionLibrary|SendAbilityActivateabletoUI self "(TagName=\"InputTag.SpecialAbility.ForcePush\")" "(TagName=\"Player.Cooldown.SpecialAbility.ForcePush\")")
                  (Class|MWBlueprintFunctionLibrary|SendAbilityActivateabletoUI self "(TagName=\"InputTag.SpecialAbility.Ult\")" "(TagName=\"Player.Cooldown.SpecialAbility.Ult\")"))))
            (:Added
              (Class|MWBlueprintFunctionLibrary|SendAbilityDisabletoUI self "(TagName=\"InputTag.SpecialAbility.Slam\")")
              (Class|MWBlueprintFunctionLibrary|SendAbilityDisabletoUI self "(TagName=\"InputTag.SpecialAbility.ForcePush\")")
              (Class|MWBlueprintFunctionLibrary|SendAbilityDisabletoUI self "(TagName=\"InputTag.SpecialAbility.Ult\")"))))
        (:Added
          (Class|MWBlueprintFunctionLibrary|SendAbilityActivateabletoUI self "(TagName=\"InputTag.SpecialAbility.Slam\")" "(TagName=\"Player.Cooldown.SpecialAbility.Slam\")"))))
    (:Added
      (Class|MWBlueprintFunctionLibrary|SendAbilityDisabletoUI self "(TagName=\"InputTag.SpecialAbility.Slam\")"))))

(event Collision|EventActorBeginOverlap
  (params (OtherActor :type Actor%20Object%20Reference)))

(event EventTick
  (params (DeltaSeconds :type Float%20%28single-precision%29)))

(fn ConstructionScript)