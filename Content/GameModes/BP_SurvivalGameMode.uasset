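; Survival game mode Blueprint that drives the wave announcement UI and end-of-game screens.
; On BeginPlay it binds to the survival state change event and switches on the state, creating wave text widgets with or without a countdown.
; When all waves finish or the player dies, it deletes the saved game slot, clears widgets, fades the camera, then async loads and shows the win or lose screen.
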(event Custom|OnSurvivalGameModeStateChanged_Event
  (params (CurrentState :type EMWSurvivalGameModeState%20Enum :default "WaitSpawnNewWave"))
  (switch Utilities|FlowControl|Switch|SwitchonEMWSurvivalGameModeState CurrentState
    (:WaitSpawnNewWave
      (CallFunction|CreateWaveWidgetwithCountdown "New Wave Coming In" (Variables|Default|GetSpawnNewWaveWaitTime)))
    (:SpawningNewWave
      (CallFunction|CreateWaveWidgetNoCountdown (Utilities|Text|FormatText "Wave {CurrentWaveCount}" (Variables|Default|GetCurrentWaveCount))))
    (:WaveCompleted
      (CallFunction|CreateWaveWidgetwithCountdown (Utilities|Text|FormatText "Wave {CurrentWaveCount} Completed" (Variables|Default|GetCurrentWaveCount)) (Variables|Default|GetWaveCompletedWaitTime)))
    (:AllWavesDone
      (Class|MWBlueprintFunctionLibrary|TryDeleteSavedGameinSlot "(TagName=\"GameData.SaveGame.Slot.2\")")
      (Utilities|FlowControl|Delay 1.0)
      (Viewport|RemoveAllWidgets)
      (CameraFades|StartCameraFade :self (Game|GetPlayerCameraManager 0) :ToAlpha 1.0 :Duration 3.0 :bHoldWhenFinished true)
      (Utilities|FlowControl|Delay 3.0)
      (bind _class (Utilities|AsyncLoadClassAsset "/Game/Widget/GameModeWidgets/WBP_WinScreen.WBP_WinScreen_C")
        (:Completed
          (bind _asuser_widget (Utilities|Casting|CastToUserWidgetClass _class))
          (bind _returnvalue (UserInterface|CreateWidget _asuser_widget))
          (UserInterface|Viewport|AddtoViewport _returnvalue 0))))
    (:PlayerDied
      (Class|MWBlueprintFunctionLibrary|TryDeleteSavedGameinSlot "(TagName=\"GameData.SaveGame.Slot.2\")")
      (Viewport|RemoveAllWidgets)
      (CameraFades|StartCameraFade :self (Game|GetPlayerCameraManager 0) :ToAlpha 1.0 :Duration 2.0 :bHoldWhenFinished true)
      (Utilities|FlowControl|Delay 2.0)
      (bind _class_2 (Utilities|AsyncLoadClassAsset "/Game/Widget/GameModeWidgets/WBP_LoseScreen.WBP_LoseScreen_C")
        (:Completed
          (bind _asuser_widget_2 (Utilities|Casting|CastToUserWidgetClass _class_2))
          (bind _returnvalue_2 (UserInterface|CreateWidget _asuser_widget_2))
          (UserInterface|Viewport|AddtoViewport _returnvalue_2 0))))))

(event EventBeginPlay
  (EventDispatchers|AssignOnSurvivalGameModeStateChanged (delegate Custom|OnSurvivalGameModeStateChanged_Event)))

(event EventTick
  (params (DeltaSeconds :type Float%20%28single-precision%29)))

(fn ConstructionScript)

(fn CreateWaveWidgetwithCountdown
  (params (TextToDisplay :type Text) (InTotalCountdownTime :type Float%20%28single-precision%29))
  (bind _returnvalue (UserInterface|CreateWidget "/Game/Widget/GameModeWidgets/WBP_WaveTextWithCountdown.WBP_WaveTextWithCountdown_C"))
  (UserInterface|Viewport|AddtoViewport _returnvalue 0)
  (Rendering|Components|TextRender|SetText (Variables|/Game/Widget/GameModeWidgets/WBP_WaveTextWithCountdown.WBP_WaveTextWithCountdown_C|GetTextBlock_WaveText _returnvalue) TextToDisplay)
  (Default|StartCountdown _returnvalue InTotalCountdownTime))

(fn CreateWaveWidgetNoCountdown
  (params (TextToDisplay :type Text))
  (bind _returnvalue (UserInterface|CreateWidget "/Game/Widget/GameModeWidgets/WBP_WaveTextNoCountdown.WBP_WaveTextNoCountdown_C"))
  (UserInterface|Viewport|AddtoViewport _returnvalue 0)
  (Rendering|Components|TextRender|SetText (Variables|/Game/Widget/GameModeWidgets/WBP_WaveTextNoCountdown.WBP_WaveTextNoCountdown_C|GetTextBlock_WaveText _returnvalue) TextToDisplay))